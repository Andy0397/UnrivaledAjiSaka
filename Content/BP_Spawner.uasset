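; BP_Spawner is a timer-driven spawner actor that, as wired, only counts and prints seconds.
; BeginPlay starts a looping one-second timer on the Spawner event, which increments Time and prints it.
; A disconnected chain, which never runs, holds a decrement, a zero check on Time, an AI spawn of BP_Siluman at the actor's location and a timer pause.
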(event Custom|Spawner
  (bind _time (Variables|Default|GetTime))
  (Math|Float|IncrementFloat _time
    (:%20%20
      (Development|PrintString (Utilities|String|ToString(Float) _time)))))

(event EventBeginPlay
  (bind _returnvalue (Utilities|Time|SetTimerbyEvent (delegate Custom|Spawner) 1.0 true))
  (Variables|Default|SetTimerHandler _returnvalue))

(fn ConstructionScript)