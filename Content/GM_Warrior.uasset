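; GM_Warrior is a game mode that starts background music and hands input to the player when play begins.
; BeginPlay calls SetMusic, then enables input on the first player controller and switches it to game-only input mode.
; SetMusic either creates, stores and plays a 2D BGM sound or stops it, based on its Play flag.
; An unconnected snippet that clears GameOver on BP_Aji_Saka never runs.
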(event EventBeginPlay
  (bind _returnvalue (Game|GetPlayerController 0))
  (CallFunction|SetMusic true)
  (Input|EnableInput _returnvalue 0)
  (Input|SetInputModeGameOnly _returnvalue))

(fn ConstructionScript)

(fn SetMusic
  (params (Play :type Boolean))
  (if Play
    (bind _returnvalue (Audio|CreateSound2D "/Game/Sound/BGM/BGM.BGM" 1.0 1.0 0.0 0))
    (bind _output_get (Variables|Default|SetBGM _returnvalue))
    (Audio|Components|Audio|Play _output_get 0.0)
    (else
      (Audio|Components|Audio|Stop (Variables|Default|GetBGM)))))