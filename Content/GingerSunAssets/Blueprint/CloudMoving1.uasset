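; Cloud actor that moves a paper sprite along a spline path in the level.
; On BeginPlay it finds a SplinePathBP1 actor, sets the sprite to opaque white and plays a timeline scaled to TimetoCompleteInSecond.
; Each update lerps along the spline length, setting actor location in world space and rotation from the spline's local space.
; An older offset-based movement timeline and a translucent tint are left unconnected.
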(event Custom|MoveObject
  (bind _splineref2 (Variables|Default|GetSplineREF2))
  (bind _spline (Variables|/Game/GingerSunAssets/Blueprint/SplinePathBP1.SplinePathBP1_C|GetSpline _splineref2))
  (Sprite|SetSpriteColor (Variables|Default|GetPaperSprite) "(R=1.000000,G=1.000000,B=1.000000,A=1.000000)")
  (Components|Timeline|SetPlayRate (Variables|Default|GetMoveObjectT) (/ 1.0 (Variables|Default|GetTimetoComplete%28inSecond%29)))
  (bind _movetrack (Timeline|MoveObjectT Play)
    (:Update
      (Transformation|SetActorTransform (Math|Transform|MakeTransform (Spline|GetLocationatDistanceAlongSpline _spline (Math|Float|Lerp 0.0 (Spline|GetSplineLength (Variables|/Game/GingerSunAssets/Blueprint/SplinePathBP1.SplinePathBP1_C|GetSpline (Variables|Default|GetSplineREF2))) _movetrack) "World") (Spline|GetRotationatDistanceAlongSpline _spline (Math|Float|Lerp 0.0 (Spline|GetSplineLength (Variables|/Game/GingerSunAssets/Blueprint/SplinePathBP1.SplinePathBP1_C|GetSpline (Variables|Default|GetSplineREF2))) _movetrack) "Local") "1.000000,1.000000,1.000000")))))

(event EventBeginPlay
  (bind _returnvalue (Actor|GetActorOfClass "/Game/GingerSunAssets/Blueprint/SplinePathBP1.SplinePathBP1_C"))
  (Variables|Default|SetSplineREF2 _returnvalue)
  (CallFunction|MoveObject))

(event Collision|EventActorBeginOverlap
  (params (OtherActor :type Actor%20Object%20Reference)))

(event EventTick
  (params (DeltaSeconds :type Float%20%28single-precision%29)))

(fn ConstructionScript)