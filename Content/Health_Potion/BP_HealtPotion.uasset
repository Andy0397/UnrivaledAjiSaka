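; Health potion pickup that restores the player's BP_Aji_Saka character when it overlaps the Box trigger.
; An overlap by player 0 plays the drink sound, removes the trigger and calls PlayDamage on the Inc_HP_15 widget.
; It then adds a fixed amount to HP, or to Armor if HP is already full, caps the result and destroys itself after a short delay.
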(event OnComponentBeginOverlap(Box)
  (params (OverlappedComponent :type Primitive%20Component%20Object%20Reference) (OtherActor :type Actor%20Object%20Reference) (OtherComp :type Primitive%20Component%20Object%20Reference) (OtherBodyIndex :type Integer) (bFromSweep :type Boolean) (SweepResult :type Hit%20Result%20Structure%20%28by%20ref%29))
  (bind _asbp_aji_saka (Utilities|Casting|CastToBP_Aji_Saka OtherActor))
  (Variables|Default|SetAs%20BP%20Warrior _asbp_aji_saka)
  (if (== OtherActor (Game|GetPlayerCharacter 0))
    (Audio|PlaySound2D "/Game/Sound/SFX/SFX_PotionDrink.SFX_PotionDrink" 1.0 1.0 0.0 0 0)
    (Components|DestroyComponent (Variables|Default|GetBox))
    (bind _foundwidgets (Widget|GetAllWidgetsOfClass "/Game/Aji_Saka/Inc_HP_15.Inc_HP_15_C" false))
    (Default|PlayDamage (Utilities|Array|Get(acopy) _foundwidgets))
    (if (< (Variables|/Game/Aji_Saka/BP_Aji_Saka.BP_Aji_Saka_C|GetHP (Variables|Default|GetAs%20BP%20Warrior)) 1e+02)
      (bind _output_get (Variables|/Game/Aji_Saka/BP_Aji_Saka.BP_Aji_Saka_C|SetHP (Variables|Default|GetAs%20BP%20Warrior) (+ (Variables|/Game/Aji_Saka/BP_Aji_Saka.BP_Aji_Saka_C|GetHP (Variables|Default|GetAs%20BP%20Warrior)) 15.0)))
      (if (>= _output_get 1e+02)
        (Variables|/Game/Aji_Saka/BP_Aji_Saka.BP_Aji_Saka_C|SetHP (Variables|Default|GetAs%20BP%20Warrior) 1e+02))
      (else
        (bind _output_get_2 (Variables|/Game/Aji_Saka/BP_Aji_Saka.BP_Aji_Saka_C|SetArmor (Variables|Default|GetAs%20BP%20Warrior) (+ (Variables|/Game/Aji_Saka/BP_Aji_Saka.BP_Aji_Saka_C|GetArmor (Variables|Default|GetAs%20BP%20Warrior)) 15.0)))
        (if (>= _output_get_2 1e+02)
          (Variables|/Game/Aji_Saka/BP_Aji_Saka.BP_Aji_Saka_C|SetArmor (Variables|Default|GetAs%20BP%20Warrior) 1e+02))))
    (Utilities|FlowControl|Delay 1.0)
    (Actor|DestroyActor)))

(event Custom|CustomEvent
  (params (OverlappedComponent :type Primitive%20Component%20Object%20Reference) (OtherActor :type Actor%20Object%20Reference) (OtherComp :type Primitive%20Component%20Object%20Reference) (OtherBodyIndex :type Integer) (bFromSweep :type Boolean) (SweepResult :type Hit%20Result%20Structure%20%28by%20ref%29)))

(event EventBeginPlay)

(event Collision|EventActorBeginOverlap
  (params (OtherActor :type Actor%20Object%20Reference)))

(event EventTick
  (params (DeltaSeconds :type Float%20%28single-precision%29)))

(fn ConstructionScript)