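; BP_Prajurit is a sprite-based enemy soldier that chases the player (BP_Aji_Saka) and plays an attack animation on reaching them.
; PawnSensing triggers AIMoveTo, while Tick flips the sprite by actor rotation from X velocity.
; Damage triggers a hit animation and knockback launch.
; Death increments the player's KillCount, rolls for health potion drops at random reachable points nearby, then destroys the actor after a delay.
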(event OnSeePawn(PawnSensing)
  (params (Pawn :type Pawn%20Object%20Reference))
  (Variables|Default|SetIsSeeEnemy? true)
  (CallFunction|FollowPlayer))

(event Custom|FollowPlayer
  (Variables|Default|SetCanAttack? true)
  (if (Variables|Default|GetIsSeeEnemy?)
    (AI|AIMoveTo self "0, 0, 0" (Game|GetPlayerCharacter 0) 5e+01 false
      (:OnSuccess
        (if (not (Variables|/Game/Aji_Saka/BP_Aji_Saka.BP_Aji_Saka_C|GetGameOver? (Variables|Default|GetPlayerRef)))
          (if (Variables|Default|GetCanAttack?)
            (Class|PaperZDAnimInstance|JumptoNode (Variables|/Script/PaperZD.PaperZDAnimationComponent|GetAnimInstance (Variables|Default|GetAnimationComponent)) "ATK" "None")
            (Utilities|FlowControl|Delay 0.2)
            (Variables|Default|SetCanAttack? false)))))
    (else
      (Variables|Default|SetIsSeeEnemy? false))))

(event Custom|FlipSprite
  (Transformation|SetActorRotation (Math|Rotator|SelectRotator "0, 0, 0" "0,180.000000, 0" (Variables|Default|GetIsMovingRight?))))

(event Custom|Drop%20item
  (bind _charactermovement (Variables|Character|GetCharacterMovement))
  (bind _returnvalue (Class|CharacterMovementComponent|GetLastUpdateLocation _charactermovement))
  (bind _outhit (Collision|LineTraceByChannel _returnvalue (- _returnvalue "0,0,200.000000") "TraceTypeQuery1" false (Utilities|Array|MakeArray (Game|GetPlayerCharacter 0)) "None" true "(R=1.000000,G=0.000000,B=0.000000,A=1.000000)" "(R=0.000000,G=1.000000,B=0.000000,A=1.000000)" 1e+09))
  (Game|SpawnActorfromClass (Utilities|Select :Index (Math|Random|RandomIntegerinRange 0 2) :Option%200 0 :Option%201 "/Game/Health_Potion/BP_HealtPotion.BP_HealtPotion_C" :Option%202 0 :Option%203 0) (Math|Transform|MakeTransform (.RandomLocation (AI|Navigation|GetRandomReachablePointinRadius (.Location (Collision|BreakHitResult _outhit)) 2e+02 0 0))) "AdjustIfPossibleButDontSpawnIfColliding" 0 0))

(event Custom|UpdateRotation
  (Utilities|IsValid (AI|GetAIController self)
    (:Is%20Valid
      (Math|Float|CompareFloat (.X (Math|Vector|BreakVector (Variables|/Script/Engine.MovementComponent|GetVelocity (Variables|Character|GetCharacterMovement)))) 0.0
        (:>
          (Variables|Default|SetIsMovingRight? true))
        (:<
          (Variables|Default|SetIsMovingRight? false))))))

(event EventBeginPlay
  (bind _returnvalue (Actor|GetActorOfClass "/Game/Aji_Saka/BP_Aji_Saka.BP_Aji_Saka_C"))
  (Variables|Default|SetPlayerRef _returnvalue))

(event EventTick
  (params (DeltaSeconds :type Float%20%28single-precision%29))
  (CallFunction|UpdateRotation)
  (CallFunction|FlipSprite))

(event Game|Damage|EventAnyDamage
  (params (Damage :type Float%20%28single-precision%29) (DamageType :type Damage%20Type%20Object%20Reference) (InstigatedBy :type Controller%20Object%20Reference) (DamageCauser :type Actor%20Object%20Reference))
  (bind _animationcomponent (Variables|Default|GetAnimationComponent))
  (bind _playerref (Variables|Default|GetPlayerRef))
  (bind _animinstance (Variables|/Script/PaperZD.PaperZDAnimationComponent|GetAnimInstance _animationcomponent))
  (bind _output_get (Variables|Default|SetHP (- (Variables|Default|GetHP) Damage)))
  (if (<= _output_get 0.0)
    (Components|DestroyComponent (Variables|Default|GetCapsuleComponent))
    (Class|PaperZDAnimInstance|JumptoNode _animinstance "DEAD" "None")
    (Variables|/Game/Aji_Saka/BP_Aji_Saka.BP_Aji_Saka_C|SetKillCount _playerref (+ (Variables|/Game/Aji_Saka/BP_Aji_Saka.BP_Aji_Saka_C|GetKillCount _playerref) 1))
    (for _index (range 0 1)
      (CallFunction|DropItem))
    (Utilities|FlowControl|Delay 1.5)
    (Actor|DestroyActor)
    (else
      (Class|PaperZDAnimInstance|JumptoNode _animinstance "HIT" "None")
      (Character|LaunchCharacter (* (Transformation|GetActorForwardVector) (Variables|Default|GetKnockBack)) false false))))

(fn ConstructionScript)